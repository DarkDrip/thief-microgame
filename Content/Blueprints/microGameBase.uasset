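; Base Blueprint for swipe-driven microgames that picks one of four games at random.
; RandomMicro rolls a game, blends the player's view to the CameraActor tagged for it and records CurrentGame.
; CastChar caches the owning BP_ThirdPersonCharacter for swipe-direction checks that print completion.
; Those checks, a duplicate picker and the RandomMicro call are disconnected; the fourth check tests game 3 instead of 4.
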(event Custom|CastChar
  (bind _asbp_third_person_character (Utilities|Casting|CastToBP_ThirdPersonCharacter (Components|GetOwner)))
  (Variables|Default|SetAs%20BP%20Third%20Person%20Character_1 _asbp_third_person_character))

(event EventBeginPlay)

(event Collision|EventActorBeginOverlap
  (params (OtherActor :type Actor%20Object%20Reference)))

(event EventTick
  (params (DeltaSeconds :type Float%20%28single-precision%29)))

(fn ConstructionScript)

(fn RandomMicro
  (bind _output_get (Variables|Default|SetrandomGame (Math|Random|RandomInteger 4)))
  (Development|PrintString (Utilities|String|ToString(Integer) _output_get))
  (Utilities|FlowControl|Sequence
    (:then_0
      (if (== _output_get 0)
        (bind _outactors (Actor|GetAllActorsOfClasswithTag "/Script/Engine.CameraActor" "Game1"))
        (for _array_element _outactors
          (Game|Player|SetViewTargetwithBlend (Game|GetPlayerController 0) _array_element 0.0 "VTBlend_Linear" 0.0 false)
          (Variables|Default|SetCurrentGame 1))))
    (:then_1
      (if (== _output_get 1)
        (bind _outactors_2 (Actor|GetAllActorsOfClasswithTag "/Script/Engine.CameraActor" "Game2"))
        (for _array_element_2 _outactors_2
          (Game|Player|SetViewTargetwithBlend (Game|GetPlayerController 0) _array_element_2 0.0 "VTBlend_Linear" 0.0 false)
          (Variables|Default|SetCurrentGame 2))))
    (:then_2
      (if (== _output_get 2)
        (bind _outactors_3 (Actor|GetAllActorsOfClasswithTag "/Script/Engine.CameraActor" "Game3"))
        (for _array_element_3 _outactors_3
          (Game|Player|SetViewTargetwithBlend (Game|GetPlayerController 0) _array_element_3 0.0 "VTBlend_Linear" 0.0 false)
          (Variables|Default|SetCurrentGame 3))))
    (:then_3
      (if (== _output_get 3)
        (bind _outactors_4 (Actor|GetAllActorsOfClasswithTag "/Script/Engine.CameraActor" "Game4"))
        (for _array_element_4 _outactors_4
          (Game|Player|SetViewTargetwithBlend (Game|GetPlayerController 0) _array_element_4 0.0 "VTBlend_Linear" 0.0 false)
          (Variables|Default|SetCurrentGame 4))))))